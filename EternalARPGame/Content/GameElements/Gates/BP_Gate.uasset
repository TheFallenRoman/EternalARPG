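; Double gate actor that swings open when a Character enters its trigger box and closes when one leaves.
; OpenGates and CloseGates play two timelines forward or in reverse, yawing the left and right door scenes up to 90 degrees in opposite directions.
; Each call restarts from the track's start or end rather than its current position.
; The construction script applies AnimationPlayRate to both timelines.
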(event OnComponentBeginOverlap(GateTriggerBox)
  (params (OverlappedComponent :type Primitive%20Component%20Object%20Reference) (OtherActor :type Actor%20Object%20Reference) (OtherComp :type Primitive%20Component%20Object%20Reference) (OtherBodyIndex :type Integer) (bFromSweep :type Boolean) (SweepResult :type Hit%20Result%20Structure%20%28by%20ref%29))
  (Utilities|Casting|CastToCharacter OtherActor)
  (CallFunction|OpenGates))

(event OnComponentEndOverlap(GateTriggerBox)
  (params (OverlappedComponent :type Primitive%20Component%20Object%20Reference) (OtherActor :type Actor%20Object%20Reference) (OtherComp :type Primitive%20Component%20Object%20Reference) (OtherBodyIndex :type Integer))
  (Utilities|Casting|CastToCharacter OtherActor)
  (CallFunction|CloseGates))

(event Custom|OpenGates
  ;[1 1 1] Open/Close the left and right gate doors at the same time using a timline to make the transition smooth.
  (Utilities|FlowControl|Sequence
    (:then_0
      (bind _opentrackalpha (Timeline|OpenRightGateTimeline PlayFromStart)
        (:Update
          (Transformation|SetRelativeRotation (Variables|Default|GetRightDoorScene) (Math|Rotator|MakeRotator 0.0 0.0 (* _opentrackalpha 9e+01)) false false))))
    (:then_1
      (bind _opentrackalpha_2 (Timeline|OpenLeftGateTimeline PlayFromStart)
        (:Update
          (Transformation|SetRelativeRotation (Variables|Default|GetLeftDoorScene) (Math|Rotator|MakeRotator 0.0 0.0 (* _opentrackalpha_2 -9e+01)) false false))))))

(event Custom|CloseGates
  ;[1 1 1] Open/Close the left and right gate doors at the same time using a timline to make the transition smooth.
  (Utilities|FlowControl|Sequence
    (:then_0
      (bind _opentrackalpha (Timeline|OpenRightGateTimeline ReverseFromEnd)
        (:Update
          (Transformation|SetRelativeRotation (Variables|Default|GetRightDoorScene) (Math|Rotator|MakeRotator 0.0 0.0 (* _opentrackalpha 9e+01)) false false))))
    (:then_1
      (bind _opentrackalpha_2 (Timeline|OpenLeftGateTimeline ReverseFromEnd)
        (:Update
          (Transformation|SetRelativeRotation (Variables|Default|GetLeftDoorScene) (Math|Rotator|MakeRotator 0.0 0.0 (* _opentrackalpha_2 -9e+01)) false false))))))

(event EventBeginPlay)

(fn ConstructionScript
  (Components|Timeline|SetPlayRate (Variables|Default|GetOpenRightGateTimeline) (Variables|Default|GetAnimationPlayRate)))