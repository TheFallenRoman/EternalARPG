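; BP_Platform is a moving platform that travels back and forth along designer-set points, pausing at its turnaround points.
; The construction script adds each MovementLocationPoints entry to an InterpToMovementComponent as a relative control point.
; BeginPlay activates that component after a delay of SecondsToWaitAtTurnAroundPoints.
; On each reverse event, it disables the component's tick for the same delay, then re-enables it to resume movement.
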(event OnInterptoReverse(InterptoMovementComponent)
  (params (ImpactResult :type Hit%20Result%20Structure%20%28by%20ref%29) (Time :type Float%20%28single-precision%29))
  ;[1 1 1] When platform hits a turn around point, delay its movment for a number of seconds.
  (Components|Tick|SetComponentTickEnabled (Variables|Default|GetInterp%20to%20Movement%20Component) false)
  (Utilities|FlowControl|Delay (Variables|Default|GetSecondsToWaitAtTurnAroundPoints))
  (Components|Tick|SetComponentTickEnabled (Variables|Default|GetInterp%20to%20Movement%20Component) true))

(event EventBeginPlay
  ;[1 1 1] Halt movment of platforms for a short time before activating them.
  (Utilities|FlowControl|Delay (Variables|Default|GetSecondsToWaitAtTurnAroundPoints))
  (Components|Activation|Activate (Variables|Default|GetInterp%20to%20Movement%20Component) false))

(fn ConstructionScript
  (for _array_element (Variables|Default|GetMovementLocationPoints)
    (Class|InterptoMovementComponent|AddControlPointPosition (Variables|Default|GetInterp%20to%20Movement%20Component) _array_element true)))