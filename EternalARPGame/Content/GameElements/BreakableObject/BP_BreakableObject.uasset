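; BP_BreakableObject is a breakable world actor that loses hit points from any damage and breaks apart at zero.
; Each hit plays a camera shake centered on the player, and non-lethal hits briefly run an InterpToMovement component through tick toggling and a retriggerable delay.
; On destruction it stops that movement, calls CETrigger on its FS_MasterField child actor and expires after a short life span.
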(event Custom|DestroyObject
  (Components|Tick|SetComponentTickEnabled (Variables|Default|GetInterpToMovement) false)
  (bind _asfs_master_field (Utilities|Casting|CastToFS_MasterField (Variables|/Script/Engine.ChildActorComponent|GetChildActor (Variables|Default|GetFS_Master_Field))))
  (Default|CETrigger _asfs_master_field)
  (Actor|SetLifeSpan 3.0))

(event EventBeginPlay
  (Components|Tick|SetComponentTickEnabled (Variables|Default|GetInterpToMovement) false))

(event Game|Damage|EventAnyDamage
  (params (Damage :type Float%20%28single-precision%29) (DamageType :type Damage%20Type%20Object%20Reference) (InstigatedBy :type Controller%20Object%20Reference) (DamageCauser :type Actor%20Object%20Reference))
  (Camera|PlayWorldCameraShake "/Game/Core/Characters/Fiona_Wesrose/BP_CameraShake_PlayerAttack.BP_CameraShake_PlayerAttack_C" (Transformation|GetActorLocation (Game|Player|GetPlayerPawn 0)) 1e+03 3e+03)
  (bind _output_get (Variables|Default|SetHitPoints (Math|Float|Truncate (- (Variables|Default|GetHitPoints) Damage))))
  (if (<= _output_get 0)
    (Utilities|FlowControl|DoOnce false
      (:Completed
        (CallFunction|DestroyObject)))
    (else
      (Components|Tick|SetComponentTickEnabled (Variables|Default|GetInterpToMovement) true)
      (Utilities|FlowControl|RetriggerableDelay 0.2)
      (Components|Tick|SetComponentTickEnabled (Variables|Default|GetInterpToMovement) false)))
  ;[1 1 1] Delete when done
  (Development|PrintString (Utilities|String|ToString(Integer) (Variables|Default|GetHitPoints))))

(fn ConstructionScript)