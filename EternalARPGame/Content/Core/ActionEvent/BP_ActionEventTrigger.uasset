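; BP_ActionEventTrigger is an interactable trigger that moves the interacting actor along a spline, intended as a smooth cliff jump-down for the player.
; Overlapping its TriggerBox registers it as the main character's interactable object, and leaving clears it.
; On interaction, a timeline with a duration-scaled play rate drives an alpha that sets the actor's swept location along the spline each update.
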(event OnComponentBeginOverlap(TriggerBox)
  (params (OverlappedComponent :type Primitive%20Component%20Object%20Reference) (OtherActor :type Actor%20Object%20Reference) (OtherComp :type Primitive%20Component%20Object%20Reference) (OtherBodyIndex :type Integer) (bFromSweep :type Boolean) (SweepResult :type Hit%20Result%20Structure%20%28by%20ref%29))
  (bind _asbp_main_character (Utilities|Casting|CastToBP_MainCharacter OtherActor))
  (Default|SetNewInteractableObject _asbp_main_character self))

(event OnComponentEndOverlap(TriggerBox)
  (params (OverlappedComponent :type Primitive%20Component%20Object%20Reference) (OtherActor :type Actor%20Object%20Reference) (OtherComp :type Primitive%20Component%20Object%20Reference) (OtherBodyIndex :type Integer))
  (bind _asbp_main_character (Utilities|Casting|CastToBP_MainCharacter OtherActor))
  (Default|ClearCurrentInteractableObject _asbp_main_character self))

(event EventBeginPlay)

(event Collision|EventActorBeginOverlap
  (params (OtherActor :type Actor%20Object%20Reference)))

(event EventTick
  (params (DeltaSeconds :type Float%20%28single-precision%29)))

(event EventInteractwithObject
  (params (ActorSendingInteraction :type Actor%20Object%20Reference))
  ;[1 1 1] Have player jump down a cliff smoothly
  (Components|Timeline|SetPlayRate (Variables|Default|GetCharacterJumpDownLedgeTimeline) (/ 1.0 (Variables|Default|GetMovementAnimePlayrateInSeconds)))
  (bind _jumppathalpha (Timeline|CharacterJumpDownLedgeTimeline PlayFromStart)
    (:Update
      (Transformation|SetActorLocation ActorSendingInteraction (Spline|GetLocationatTime (Variables|Default|GetSpline) _jumppathalpha "World" false) true false))))

(fn ConstructionScript)