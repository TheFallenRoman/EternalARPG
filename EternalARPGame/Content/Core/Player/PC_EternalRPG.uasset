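; Player controller for EternalRPG that turns input into pawn movement and actions.
; While the move action is held, Tick traces under the cursor on the Visibility channel and moves the pawn toward the hit point.
; Axis inputs also move the pawn along fixed world directions.
; Interaction, dash and primary attack presses are forwarded as interface messages when the pawn implements BPI_InteractionActions or BPI_CharacterActions.
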(event EventTick
  (params (DeltaSeconds :type Float%20%28single-precision%29))
  (bind _returnvalue (Pawn|GetControlledPawn))
  (bind (_hitresult _returnvalue_2) (Game|Player|GetHitResultUnderCursorbyChannel "TraceTypeQuery1" true))
  ;[1 1 1] Move character in the direction that the cursor is pointed at.
  (if (and (Variables|Default|GetIsMoveActionEnabled) _returnvalue_2)
    (Pawn|Input|AddMovementInput _returnvalue (Math|Vector|GetUnitDirection(Vector) (Transformation|GetActorLocation _returnvalue) (.Location (Collision|BreakHitResult _hitresult))) 1.0 false)))

(event Input|ActionEvents|InputActionMoveAction
  (params (Key :type Key%20Structure :default "None"))
  (:Pressed
    (Variables|Default|SetIsMoveActionEnabled true))
  (:Released
    (Variables|Default|SetIsMoveActionEnabled false)))

(event Input|ActionEvents|InputActionInteraction
  (params (Key :type Key%20Structure :default "None"))
  (bind _returnvalue (Pawn|GetControlledPawn))
  (:Pressed
    ;[1 1 1] Check if the controlled pawn has the interact interface implimented then send message if true.
    (if (Utilities|DoesObjectImplementInterface _returnvalue "/Game/Core/Player/BPI_InteractionActions.BPI_InteractionActions_C")
      (Class|BPIInteractionActions|Interact(Message) _returnvalue))))

(event Input|ActionEvents|InputActionDash
  (params (Key :type Key%20Structure :default "None"))
  (bind _returnvalue (Pawn|GetControlledPawn))
  (:Pressed
    (if (Utilities|DoesObjectImplementInterface _returnvalue "/Game/Core/Player/BPI_CharacterActions.BPI_CharacterActions_C")
      (Class|BPICharacterActions|Dash(Message) _returnvalue))))

(event Input|ActionEvents|InputActionPrimaryAttack
  (params (Key :type Key%20Structure :default "None"))
  (bind _returnvalue (Pawn|GetControlledPawn))
  (:Pressed
    (if (Utilities|DoesObjectImplementInterface _returnvalue "/Game/Core/Player/BPI_CharacterActions.BPI_CharacterActions_C")
      (Class|BPICharacterActions|PrimaryAttack(Message) _returnvalue))))

(event Input|AxisEvents|InputAxisMoveUp
  (params (AxisValue :type Float%20%28single-precision%29))
  (Pawn|Input|AddMovementInput (Pawn|GetControlledPawn) "0,-1.000000, 0" AxisValue false))

(event Input|AxisEvents|InputAxisMoveRight
  (params (AxisValue :type Float%20%28single-precision%29))
  (Pawn|Input|AddMovementInput (Pawn|GetControlledPawn) "1.000000, 0, 0" AxisValue false))

(fn ConstructionScript)