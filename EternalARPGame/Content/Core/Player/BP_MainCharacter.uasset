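; Player character Blueprint handling cursor-aimed dashing, melee combos and object interaction.
; Dash and attack snap rotation toward the cursor; attacks chain numbered montage sections through a notify-opened combo window, with recovery montages on blend-out.
; While attacking, Tick sphere-traces between sword sockets and damages each actor once per swing via a hit list.
; Interact messages the stored object through BPI_InteractionActions; setter and clear functions toggle its text prompt.
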(event EventBeginPlay)

(event EventInteract
  ;[1 1 1] Ensure object reference is valid, ensure it impliments the needed interface, then send interface message.
  (Utilities|IsValid (Variables|Default|GetInteractableObjectReference)
    (:Is%20Valid
      (if (Utilities|DoesObjectImplementInterface (Variables|Default|GetInteractableObjectReference) "/Game/Core/Player/BPI_InteractionActions.BPI_InteractionActions_C")
        (Class|BPIInteractionActions|InteractwithObject(Message) (Variables|Default|GetInteractableObjectReference) self)))))

(event EventDash
  ;[1 1 1] When "SpaceBar" is hit, have player dash in the direction of the cursor.
  (if (not (Variables|Default|GetIsDashing))
    (Variables|Default|SetIsDashing true)
    (CallFunction|ChangeRotationforActions)
    (Animation|Montage|PlayMontage (Variables|Character|GetMesh) "/Game/Core/Characters/Fiona_Wesrose/AnimationMontage/AM_Dash_FionaWesrose.AM_Dash_FionaWesrose" 1.5
      (:OnCompleted
        _)
      (:OnInterrupted
        _))
    (Variables|Default|SetIsDashing false)))

(event EventPrimaryAttack
  ;[1 1 1] When "LMB" is clicked, preform Primary attack montoge and combo's
  (if (not (Variables|Default|GetIsDashing))
    (if (Variables|Default|GetIsAttacking)
      (if (Variables|Default|GetIsComboWindowOpen)
        (Math|Integer|IncrementInt (Variables|Default|GetNumberOfAttacksInCurrentCombo) :!label _label
          (:%20%20
            (Utilities|Array|Clear (Variables|Default|GetActorHitByAttack))
            (CallFunction|ChangeRotationforActions)
            (bind _notifyname (Animation|Montage|PlayMontage (Variables|Character|GetMesh) "/Game/Core/Characters/Fiona_Wesrose/AnimationMontage/AM_PrimaryAttack_FionaWesrose_Montage.AM_PrimaryAttack_FionaWesrose_Montage" 1.5 0.0 (Utilities|String|StringToName (Utilities|String|Append "PrimaryAttack_0" (Utilities|String|ToString(Integer) (Variables|Default|GetNumberOfAttacksInCurrentCombo)))))
              (:OnBlendOut
                (Variables|Default|SetIsComboWindowOpen false)
                (Animation|Montage|PlayMontage 0 "/Game/Core/Characters/Fiona_Wesrose/AnimationMontage/AM_PrimaryAttackRecovery_FionaWesrose.AM_PrimaryAttackRecovery_FionaWesrose" 1.5 0.0 (Utilities|String|StringToName (Utilities|String|Append "PrimaryAttackRecovery_0" (Utilities|String|ToString(Integer) (Variables|Default|GetNumberOfAttacksInCurrentCombo))))
                  (:then
                    (Variables|Default|SetNumberOfAttacksInCurrentCombo 0)
                    (Variables|Default|SetIsAttacking false))))
              (:OnInterrupted
                (Variables|Default|SetIsComboWindowOpen false))
              (:OnNotifyBegin
                (if (== _notifyname (Variables|Default|GetComboWindowName))
                  (Variables|Default|SetIsComboWindowOpen true)))))))
      (else
        (Variables|Default|SetIsAttacking true)
        (goto _label)))))

(event EventTick
  (params (DeltaSeconds :type Float%20%28single-precision%29))
  (bind _mesh (Variables|Character|GetMesh))
  (if (Variables|Default|GetIsAttacking)
    (bind (_outhit _returnvalue) (Collision|SphereTraceByChannel (Transformation|GetSocketLocation _mesh "Sword_Base") (Transformation|GetSocketLocation _mesh "Sword_Tip") 4e+01 "TraceTypeQuery3" false 0 "ForOneFrame"))
    (if _returnvalue
      (if (< (Utilities|Array|FindItem (Variables|Default|GetActorHitByAttack) (.HitActor (Collision|BreakHitResult _outhit))) 0)
        (Game|Damage|ApplyDamage (.HitActor (Collision|BreakHitResult _outhit)) 1.0 (Pawn|GetController) self)
        (Utilities|Array|Add (Variables|Default|GetActorHitByAttack) (.HitActor (Collision|BreakHitResult _outhit)))))))

(event Game|Damage|EventAnyDamage
  (params (Damage :type Float%20%28single-precision%29) (DamageType :type Damage%20Type%20Object%20Reference) (InstigatedBy :type Controller%20Object%20Reference) (DamageCauser :type Actor%20Object%20Reference)))

(fn ConstructionScript)

(fn SetNewInteractableObject
  (params (NewInteractableObjectReference :type Actor%20Object%20Reference))
  (Variables|Default|SetInteractableObjectReference NewInteractableObjectReference)
  (Development|SetHiddeninGame (Variables|Default|GetTextRender%28Swap%20for%20UI%29) false false))

(fn ClearCurrentInteractableObject
  (params (IncomingInteractableObjectReference :type Actor%20Object%20Reference))
  (bind _output_get (Variables|Default|SetInteractableObjectReference IncomingInteractableObjectReference))
  (if (== _output_get (Variables|Default|GetInteractableObjectReference))
    (Variables|Default|SetInteractableObjectReference 0)
    (Development|SetHiddeninGame (Variables|Default|GetTextRender%28Swap%20for%20UI%29) true false)))

(fn ChangeRotationforActions
  (bind _returnvalue (Pawn|GetController))
  (bind _returnvalue_2 (Transformation|GetActorLocation))
  (bind _aspc_eternal_rpg (Utilities|Casting|CastToPC_EternalRPG _returnvalue))
  (bind _hitresult (Game|Player|GetHitResultUnderCursorbyChannel _aspc_eternal_rpg "TraceTypeQuery1" true))
  (bind _location (Collision|BreakHitResult _hitresult))
  (bind _returnvalue_3 (Math|Vector|GetUnitDirection(Vector) _returnvalue_2 _location))
  (Transformation|SetActorRotation (Math|Conversions|RotationFromXVector (Math|Vector|MakeVector (.x _returnvalue_3) (.y _returnvalue_3) 0.0)))
  (return))